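; GI_Instance, a game instance by its name, steps the UI through a fixed sequence of screens.
; Each RemoveWidgets call checks SceneID, clears all widgets, adds the next widget to the viewport and increments the ID.
; The order runs from player select to level select to pause menu, after which further calls do nothing because no branch handles the final ID.
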(fn RemoveWidgets
  (if (== (Variables|Default|GetScene%20ID) 0)
    (Viewport|RemoveAllWidgets)
    (bind _returnvalue (UserInterface|CreateWidget "/Game/Assets/UI/WBP_PlayerSelect.WBP_PlayerSelect_C"))
    (UserInterface|Viewport|AddtoViewport _returnvalue 0)
    (Variables|Default|SetScene%20ID 1)
    (elif (== (Variables|Default|GetScene%20ID) 1)
      (Viewport|RemoveAllWidgets)
      (bind _returnvalue_2 (UserInterface|CreateWidget "/Game/Assets/UI/WBP_LevelSelect.WBP_LevelSelect_C"))
      (UserInterface|Viewport|AddtoViewport _returnvalue_2 0)
      (Variables|Default|SetScene%20ID 2)
      (elif (== (Variables|Default|GetScene%20ID) 2)
        (Viewport|RemoveAllWidgets)
        (bind _returnvalue_3 (UserInterface|CreateWidget "/Game/Assets/UI/WBP_PauseMenu.WBP_PauseMenu_C"))
        (UserInterface|Viewport|AddtoViewport _returnvalue_3 0)
        (Variables|Default|SetScene%20ID 3)))))