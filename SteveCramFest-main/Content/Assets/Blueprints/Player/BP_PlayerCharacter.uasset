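; Side-scrolling player character for two players, playing as Guitar or Flute as chosen in GI_Instance, with Tick pinning the capsule's Y position.
; The character enum routes inputs to cooldown-gated attacks: line-trace melee against "Enemy" actors, Guitar buckshot or looping Flute auto-fire.
; Movement flips the sprite and sets melee and projectile direction.
; Damage lowers Health without triggering death, and temporary debug keys swap character, load a test level or quit.
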(event EventTick
  (params (DeltaSeconds :type Float%20%28single-precision%29))
  (bind _capsulecomponent (Variables|Collision|GetCapsuleComponent))
  (bind _returnvalue (Transformation|GetWorldLocation _capsulecomponent))
  (Utilities|FlowControl|Sequence
    (:then_0
      (Transformation|SetWorldLocation _capsulecomponent (Math|Vector|MakeVector (.x _returnvalue) 5e+01 (.z _returnvalue)) false false))))

(event EventUnpossessed
  (params (OldController :type Controller%20Object%20Reference))
  (Actor|DestroyActor))

(event EventBeginPlay
  (bind _textrender (Variables|Default|GetTextRender))
  (bind _cube1 (Variables|Default|GetCube1))
  (Utilities|FlowControl|Sequence
    (:then_0
      (bind _asgi_instance (Utilities|Casting|CastToGI_Instance (Game|GetGameInstance)))
      (switch Utilities|FlowControl|Switch|SwitchonEnum_Player (Variables|Default|GetPlayer)
        (:NewEnumerator0
          (Variables|Default|SetPlayerCharacter (Variables|/Game/Assets/Blueprints/GI_Instance.GI_Instance_C|GetPlayer1Character _asgi_instance)))
        (:NewEnumerator1
          (Variables|Default|SetPlayerCharacter (Variables|/Game/Assets/Blueprints/GI_Instance.GI_Instance_C|GetPlayer2Character _asgi_instance))
          (Collision|SetCollisionEnabled _cube1 "NoCollision")
          (Rendering|SetVisibility _cube1 false false))))
    (:then_1
      (switch Utilities|FlowControl|Switch|SwitchonEnum_Character (Variables|Default|GetPlayerCharacter)
        (:NewEnumerator0
          (Rendering|Components|TextRender|SetText _textrender (Utilities|Text|MakeLiteralText "Guitar")))
        (:NewEnumerator1
          (Rendering|Components|TextRender|SetText _textrender (Utilities|Text|MakeLiteralText "Flute")))))))

(event Input|ActionEvents|InputActionMeleeAttack
  (params (Key :type Key%20Structure :default "None"))
  ;[1 1 1] Melee Attack
  (:Pressed
    (switch Utilities|FlowControl|Switch|SwitchonEnum_Character (Variables|Default|GetPlayerCharacter)
      (:NewEnumerator0
        (|GuitarMelee))
      (:NewEnumerator1
        (|FluteMelee)))))

(event Input|ActionEvents|InputActionJumping
  (params (Key :type Key%20Structure :default "None"))
  ;[1 1 1] Jumping
  (:Pressed
    (Character|Jump))
  (:Released
    (Character|StopJumping)))

(event Input|ActionEvents|InputActionRangedAttack
  (params (Key :type Key%20Structure :default "None"))
  (bind _playercharacter (Variables|Default|GetPlayerCharacter))
  ;[1 1 1] Ranged Attack
  (:Pressed
    (switch Utilities|FlowControl|Switch|SwitchonEnum_Character _playercharacter
      (:NewEnumerator0
        (|RangedAttackBuck))
      (:NewEnumerator1
        (|RangedAttackFullAuto))))
  (:Released
    (switch Utilities|FlowControl|Switch|SwitchonEnum_Character _playercharacter
      (:NewEnumerator1
        (Variables|Default|SetFluteAttacking false)))))

(event Input|ActionEvents|InputActionStart/PauseMenu
  (params (Key :type Key%20Structure :default "None"))
  ;[1 1 1] Menu Navigation
  (:Pressed
    (bind _asgi_instance (Utilities|Casting|CastToGI_Instance (Game|GetGameInstance)))
    (Default|RemoveWidgets _asgi_instance)))

(event Input|AxisEvents|InputAxisLeft/Right
  (params (AxisValue :type Float%20%28single-precision%29))
  ;[1 1 1] Left/Right Movement
  (|Movement AxisValue AxisValue AxisValue))

(event Input|GamepadEvents|GamepadRightShoulder
  (params (Key :type Key%20Structure :default "None"))
  ;[1 1 1] DEBUG - DELETE LATER
  (:Pressed
    (switch Utilities|FlowControl|Switch|SwitchonEnum_Character (Variables|Default|GetPlayerCharacter)
      (:NewEnumerator0
        (Variables|Default|SetPlayerCharacter "NewEnumerator1"))
      (:NewEnumerator1
        (Variables|Default|SetPlayerCharacter "NewEnumerator0")))))

(event Input|GamepadEvents|GamepadLeftShoulder
  (params (Key :type Key%20Structure :default "None"))
  ;[1 1 1] DEBUG - DELETE LATER
  (:Pressed
    (Game|OpenLevel(byName) "JayceeTestCharacter")))

(event Input|GamepadEvents|GamepadRightTrigger
  (params (Key :type Key%20Structure :default "None"))
  ;[1 1 1] DEBUG - DELETE LATER
  (:Pressed
    (Game|QuitGame 0 "Quit" false)))

(fn ConstructionScript)

(event Game|Damage|EventAnyDamage
  (params (Damage :type Float%20%28single-precision%29) (DamageType :type Damage%20Type%20Object%20Reference) (InstigatedBy :type Controller%20Object%20Reference) (DamageCauser :type Actor%20Object%20Reference))
  (bind _output_get (Variables|Default|SetHealth (- (Variables|Default|GetHealth) Damage)))
  (if (<= _output_get 0.0)
    _))