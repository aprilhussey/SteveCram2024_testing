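; Player's full-auto ranged projectile, a musical-note sprite that damages actors tagged Enemy.
; On BeginPlay it sets projectile movement along the X axis from a scaled Velocity variable, then randomizes the note sprite (single or double crotchet), its pitch rotation and its color.
; Sphere overlap applies Damage to enemies and destroys the projectile on any contact except actors tagged Proj or Player, which it ignores.
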(event OnComponentBeginOverlap(Sphere)
  (params (OverlappedComponent :type Primitive%20Component%20Object%20Reference) (OtherActor :type Actor%20Object%20Reference) (OtherComp :type Primitive%20Component%20Object%20Reference) (OtherBodyIndex :type Integer) (bFromSweep :type Boolean) (SweepResult :type Hit%20Result%20Structure%20%28by%20ref%29))
  (if (Actor|ActorHasTag OtherActor "Enemy")
    (Game|Damage|ApplyDamage OtherActor (Variables|Default|GetDamage) 0 self)
    (Actor|DestroyActor :!label _label)
    (elif (not (or (Actor|ActorHasTag OtherActor "Proj") (Actor|ActorHasTag OtherActor "Player")))
      (goto _label))))

(event EventBeginPlay
  (bind _papersprite (Variables|Default|GetPaperSprite))
  (Utilities|FlowControl|Sequence
    (:then_0
      (Variables|/Script/Engine.MovementComponent|SetVelocity (Variables|Default|GetProjectileMovement) (Math|Vector|MakeVector (* (Variables|Default|GetVelocity) 1.25e+03) 0.0 0.0)))
    (:then_1
      (if (Math|Random|RandomBool)
        (Rendering|Components|Sprite|SetSprite _papersprite "/Game/Assets/Blueprints/PlaceholderThings/Sprite_CrotchetWhite.Sprite_CrotchetWhite")
        (else
          (Rendering|Components|Sprite|SetSprite _papersprite "/Game/Assets/Blueprints/PlaceholderThings/Sprite_DoubleCrotchetWhite.Sprite_DoubleCrotchetWhite")))
      (Transformation|SetRelativeRotation (Variables|Default|GetPaperSprite) (Math|Rotator|MakeRotator 0.0 (Math|Random|RandomFloatinRange 0.0 3.6e+02) 0.0) false false)
      (Sprite|SetSpriteColor (Variables|Default|GetPaperSprite) (Utilities|Struct|MakeLinearColor (Math|Random|RandomFloatinRange 0.0 1.0) (Math|Random|RandomFloatinRange 0.0 1.0) (Math|Random|RandomFloatinRange 0.0 1.0) 1.0)))))

(fn ConstructionScript)